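; Dance floor panel Blueprint that flashes random colours by swapping the material on its static mesh.
; BeginPlay starts a looping timer at the Speed interval that fires the colour change event.
; Each firing switches on a random integer to set material slot 0 to a coloured material.
; RandomInteger(5) only returns 0 to 4, so the sixth option, Cyan, is never chosen.
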(event `self.ReceiveBeginPlay`
  (`KismetSystemLibrary.K2_SetTimerDelegate` (delegate `Change colour`) (`self.Speed`) true))

(event `Change colour`
  (switch `int` (`KismetMathLibrary.RandomInteger` 5)
    (:`0`
      (`PrimitiveComponent.SetMaterial` (`self.StaticMesh`) 0 (`self.Red`)))
    (:`1`
      (`PrimitiveComponent.SetMaterial` (`self.StaticMesh`) 0 (`self.Green`)))
    (:`2`
      (`PrimitiveComponent.SetMaterial` (`self.StaticMesh`) 0 (`self.Blue`)))
    (:`3`
      (`PrimitiveComponent.SetMaterial` (`self.StaticMesh`) 0 (`self.Yellow`)))
    (:`4`
      (`PrimitiveComponent.SetMaterial` (`self.StaticMesh`) 0 (`self.Pink`)))
    (:`5`
      (`PrimitiveComponent.SetMaterial` (`self.StaticMesh`) 0 (`self.Cyan`)))))

(fn `UserConstructionScript`)