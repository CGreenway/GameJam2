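; A light actor that flickers on and off at irregular intervals.
; A self-restarting timer toggles the Lit flag after a random delay of up to half a second, picking a new delay each time.
; Tick reads the flag every frame and sets the PointLight intensity to either LightIntensity or zero.
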(event `self.ReceiveBeginPlay`
  (bind _output_get (set `self.Flicker time` (`KismetMathLibrary.RandomFloatInRange` 0.0 0.5)))
  (`KismetSystemLibrary.K2_SetTimerDelegate` (delegate `Flicker`) _output_get :!label _label))

(event `Flicker`
  (if (`self.bLit`)
    (set `self.bLit` false)
    (else
      (set `self.bLit` true)))
  (set `self.Flicker time` (`KismetMathLibrary.RandomFloatInRange` 0.0 0.5))
  (goto _label))

(event `self.ReceiveTick`
  (params (DeltaSeconds :type "Float (single-precision)"))
  (bind _pointlight (`self.PointLight`))
  (if (`self.bLit`)
    (`LightComponent.SetIntensity` _pointlight (`self.LightIntensity`))
    (else
      (`LightComponent.SetIntensity` _pointlight 0.0))))

(fn `UserConstructionScript`)